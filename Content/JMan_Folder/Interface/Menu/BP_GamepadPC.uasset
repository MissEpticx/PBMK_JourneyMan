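; BP_GamepadPC is a player controller that toggles the main menu on the Menu input action.
; Each press flips MenuOpened, adds or removes the MainMenu widget, switches input mode and cursor visibility, and calls SetMovement on the kart character.
; The setup that creates the widget and caches the BP_KartChar pawn is disconnected, so this graph never assigns either reference.
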(event EventBeginPlay)

(event Input|ActionEvents|InputActionMenu
  (params (Key :type Key%20Structure :default "None"))
  (bind _self self)
  (bind _mainmenu (Variables|Default|GetMainMenu))
  (bind _playerchar (Variables|Default|GetPlayerChar))
  (:Pressed
    (if (Variables|Default|GetMenuOpened?)
      (Widget|RemovefromParent _mainmenu)
      (Input|SetInputModeGameOnly _self)
      (Variables|Default|SetbShowMouseCursor false)
      (Variables|Default|SetMenuOpened? false)
      (Default|SetMovement _playerchar false)
      (else
        (UserInterface|Viewport|AddtoViewport _mainmenu 0)
        (Input|SetInputModeGameandUI _self _mainmenu "DoNotLock" true)
        (Variables|Default|SetbShowMouseCursor true)
        (Variables|Default|SetMenuOpened? true)
        (Default|SetMovement _playerchar true)))))

(fn ConstructionScript)