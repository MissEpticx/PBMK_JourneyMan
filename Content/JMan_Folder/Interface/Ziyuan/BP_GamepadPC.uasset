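; BP_GamepadPC is a player controller Blueprint holding main menu toggle logic that is currently disconnected.
; BeginPlay is empty, and the unwired nodes that would create the MainMenu widget never run.
; A second unwired chain would use a MenuOpened flag to add or remove the menu, switching input mode and mouse cursor visibility to match.
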(event EventBeginPlay)

(fn ConstructionScript)