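; BP_RedShell is a red shell kart item that homes in on the kart one race position ahead of a given player.
; LockTarget calls HomingFunction, which searches all BP_Kart actors by PlayerPosition and, if a CloseDistance check passes, returns the target's static mesh component.
; That component becomes the ProjectileMovement homing target, with homing enabled and velocity zeroed.
; The shell destroys itself when its collision overlap matches BP_Kart.
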(event OnComponentBeginOverlap(collision)
  (params (OverlappedComponent :type Primitive%20Component%20Object%20Reference) (OtherActor :type Actor%20Object%20Reference) (OtherComp :type Primitive%20Component%20Object%20Reference) (OtherBodyIndex :type Integer) (bFromSweep :type Boolean) (SweepResult :type Hit%20Result%20Structure%20%28by%20ref%29))
  ;[0.6292 0 1] Fiona - Red shell destory
  (if (== OtherActor "/Game/JMan_Folder/Kart_Engine/Kart_BPs/BP_Kart.BP_Kart")
    (Actor|DestroyActor)))

(event Custom|LockTarget
  (params (Player :type Pawn%20Object%20Reference))
  (bind _projectilemovement (Variables|Default|GetProjectileMovement))
  ;[0.6292 0 1] Fiona - Homing Function
  (bind _asbp_kart (Utilities|Casting|CastToBP_Kart Player))
  (bind _homingt (CallFunction|HomingFunction (Variables|/Game/JMan_Folder/Kart_Engine/Kart_BPs/BP_Kart.BP_Kart_C|GetPlayer%20 _asbp_kart)))
  (Variables|/Script/Engine.ProjectileMovementComponent|SetHomingTargetComponent _projectilemovement _homingt)
  (Variables|/Script/Engine.ProjectileMovementComponent|SetbIsHomingProjectile _projectilemovement true)
  (Variables|/Script/Engine.MovementComponent|SetVelocity _projectilemovement "0, 0, 0"))

(fn ConstructionScript)

(fn HomingFunction
  (params (Player :type Pawn%20Object%20Reference))
  (bind _returnvalue (Transformation|GetActorLocation))
  (bind _returnvalue_2 (Transformation|GetActorLocation))
  (bind _returnvalue_3 (- _returnvalue_2 _returnvalue))
  (bind _returnvalue_4 (Math|Vector|VectorLength _returnvalue_3))
  ;[0.6292 0 1] Fiona - Finding which actor to lock onto and setting target
  (bind _asbp_kart (Utilities|Casting|CastToBP_Kart Player))
  (bind _outactors (Actor|GetAllActorsOfClass "/Game/JMan_Folder/Kart_Engine/Kart_BPs/BP_Kart.BP_Kart_C"))
  (bind _array_element (Utilities|Array|ForEachLoopwithBreak _outactors :!label _label)
    (:LoopBody
      (if (== (- (Variables|/Game/JMan_Folder/Kart_Engine/Kart_BPs/BP_Kart.BP_Kart_C|GetPlayer%20Position _asbp_kart) 1) (Variables|/Game/JMan_Folder/Kart_Engine/Kart_BPs/BP_Kart.BP_Kart_C|GetPlayer%20Position _array_element))
        (goto _label Break)))
    (:Completed
      (if (< _returnvalue_4 (Variables|Default|GetCloseDistance))
        (Variables|Default|SetHomingtarget _array_element)
        (Variables|Default|SetCloseDistance _returnvalue_4)
        (return (Actor|GetComponentbyClass (Variables|Default|GetHomingtarget) "/Script/Engine.StaticMeshComponent"))))))