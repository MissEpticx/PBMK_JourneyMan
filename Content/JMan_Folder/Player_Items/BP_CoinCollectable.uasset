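; BP_CoinCollectable is a coin pickup that karts collect by overlapping its sphere.
; Each pickup raises the BP_Kart's coin count and boosts both current and default max speed, until the count reaches its cap.
; Even at the cap, it clears its CoinSpawner's spawned flag, calls SpawnCoin for a replacement and destroys itself, provided the spawner cast succeeds.
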(event OnComponentBeginOverlap(Sphere)
  (params (OverlappedComponent :type Primitive%20Component%20Object%20Reference) (OtherActor :type Actor%20Object%20Reference) (OtherComp :type Primitive%20Component%20Object%20Reference) (OtherBodyIndex :type Integer) (bFromSweep :type Boolean) (SweepResult :type Hit%20Result%20Structure%20%28by%20ref%29))
  ;[0.6292 0 1] Fiona - Collecting Coin (Adds to coin count + increases max speed)/If coin count is already maxed out does nothing
  (bind _asbp_kart (Utilities|Casting|CastToBP_Kart OtherActor))
  (if (== (Variables|/Game/JMan_Folder/Kart_Engine/Kart_BPs/BP_Kart.BP_Kart_C|GetCoin%20Count _asbp_kart) 10)
    (Variables|/Game/JMan_Folder/Kart_Engine/Kart_BPs/BP_Kart.BP_Kart_C|SetCoin%20Count _asbp_kart 10)
    (else
      (Variables|/Game/JMan_Folder/Kart_Engine/Kart_BPs/BP_Kart.BP_Kart_C|SetCoin%20Count _asbp_kart (+ (Variables|/Game/JMan_Folder/Kart_Engine/Kart_BPs/BP_Kart.BP_Kart_C|GetCoin%20Count _asbp_kart) 1))
      (Variables|/Game/JMan_Folder/Kart_Engine/Kart_BPs/BP_Kart.BP_Kart_C|SetCurrent%20Speed _asbp_kart (+ (Variables|/Game/JMan_Folder/Kart_Engine/Kart_BPs/BP_Kart.BP_Kart_C|GetCurrent%20Speed _asbp_kart) 2.0))
      (Variables|/Game/JMan_Folder/Kart_Engine/Kart_BPs/BP_Kart.BP_Kart_C|SetDefault%20Max%20Speed _asbp_kart (+ (Variables|/Game/JMan_Folder/Kart_Engine/Kart_BPs/BP_Kart.BP_Kart_C|GetDefault%20Max%20Speed _asbp_kart) 2.0))))
  ;[0.6562 0.007784 0] Respawn Coin - Colette
  (bind _ascoin_spawner (Utilities|Casting|CastToCoinSpawner (Variables|Default|GetCoin%20Spawner)))
  (Variables|/Game/JMan_Folder/Player_Items/CoinSpawner.CoinSpawner_C|SetHasSpawned _ascoin_spawner false)
  (Default|SpawnCoin _ascoin_spawner)
  (Actor|DestroyActor))

(fn ConstructionScript)