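; BP_IceFlower is an Ice Flower player item that makes a kart slide at a locked speed for a short time.
; IceFlowerSlide flags the given BP_Kart as Icy, stores its current speed as IcySpeed and clears the flag after a delay.
; A looping timer reapplies IcySpeed to CurrentSpeed while the kart is Icy; nothing in this Blueprint clears that timer.
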(event Custom|IceFlowerSlide
  (params (Player :type Pawn%20Object%20Reference))
  (Utilities|Time|SetTimerbyEvent (delegate Custom|Checking%20if%20icy) 0.2 true)
  (bind _asbp_kart (Utilities|Casting|CastToBP_Kart Player))
  (Variables|/Game/JMan_Folder/Kart_Engine/Kart_BPs/Karts/BP_Kart.BP_Kart_C|SetIcy _asbp_kart true)
  (Variables|/Game/JMan_Folder/Kart_Engine/Kart_BPs/Karts/BP_Kart.BP_Kart_C|SetIcySpeed _asbp_kart (Variables|/Game/JMan_Folder/Kart_Engine/Kart_BPs/Karts/BP_Kart.BP_Kart_C|GetCurrent%20Speed _asbp_kart))
  (Utilities|FlowControl|Delay 2.0)
  (Variables|/Game/JMan_Folder/Kart_Engine/Kart_BPs/Karts/BP_Kart.BP_Kart_C|SetIcy _asbp_kart false))

(event Custom|Checking%20if%20icy
  (bind _asbp_kart (Utilities|Casting|CastToBP_Kart (stale Custom|IceFlowerSlide Player)))
  (if (Variables|/Game/JMan_Folder/Kart_Engine/Kart_BPs/Karts/BP_Kart.BP_Kart_C|GetIcy _asbp_kart)
    (Variables|/Game/JMan_Folder/Kart_Engine/Kart_BPs/Karts/BP_Kart.BP_Kart_C|SetCurrent%20Speed _asbp_kart (Variables|/Game/JMan_Folder/Kart_Engine/Kart_BPs/Karts/BP_Kart.BP_Kart_C|GetIcySpeed _asbp_kart))))

(event EventBeginPlay)

(event EventTick
  (params (DeltaSeconds :type Float%20%28single-precision%29)))

(fn ConstructionScript)