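; BP_TripleBanana is a player item actor that orbits a target actor on the horizontal plane.
; Tick advances an accumulated angle by rotation speed, clockwise or counterclockwise, and passes it to RotateActorAroundPoint.
; That function rotates a radius vector around Z by this angle plus a starting offset, then sets the actor's location around the target.
; Without a valid target, it orbits its spawn location, saved on BeginPlay.
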(event EventBeginPlay
  ;[0.6292 0 1] Fiona - Getting inital spawn location
  (Variables|Default|SetInitialLocation (Transformation|GetActorLocation)))

(event EventTick
  (params (DeltaSeconds :type Float%20%28single-precision%29))
  ;[0.6292 0 1] Fiona - Rotation around chosen actor
  (Variables|Default|SetCurrentRotation (+ (Variables|Default|GetCurrentRotation) (* (* (Variables|Default|GetRotationSpeed) DeltaSeconds) (Math|Float|SelectFloat 1.0 -1.0 (Variables|Default|GetClockwise)))))
  (CallFunction|RotateActorAroundPoint self (Variables|Default|GetTargetActor) (Variables|Default|GetInitialLocation) (Variables|Default|GetRadius) (Variables|Default|GetStartingAngle) (Variables|Default|GetCurrentRotation)))

(fn ConstructionScript)

(fn RotateActorAroundPoint
  (params (Actor%20To%20Rotate :type Actor%20Object%20Reference) (Target%20Actor :type Actor%20Object%20Reference) (Target%20Location :type Vector) (Radius :type Float%20%28single-precision%29) (Angle :type Float%20%28single-precision%29) (Rotation%20Rate :type Float%20%28single-precision%29))
  (LocalVariables|SetLActorToRotate Actor%20To%20Rotate)
  (LocalVariables|SetLTargetActor Target%20Actor)
  (LocalVariables|SetLLocation Target%20Location)
  (LocalVariables|SetLO%20Radius Radius)
  (LocalVariables|SetLAngle Angle)
  (LocalVariables|SetLRate Rotation%20Rate)
  (Utilities|IsValid (LocalVariables|GetLTargetActor)
    (:Is%20Valid
      (LocalVariables|SetLLocation (Transformation|GetActorLocation (LocalVariables|GetLTargetActor))))
    (:Is%20Not%20Valid
      _))
  (Transformation|SetActorLocation (LocalVariables|GetLActorToRotate) (+ (LocalVariables|GetLLocation) (Math|Vector|RotateVectorAroundAxis (Math|Vector|MakeVector (LocalVariables|GetLO%20Radius) 0.0 0.0) (+ (LocalVariables|GetLRate) (LocalVariables|GetLAngle)) "0, 0,1.000000")) false false)
  (return (LocalVariables|GetLLocation)))