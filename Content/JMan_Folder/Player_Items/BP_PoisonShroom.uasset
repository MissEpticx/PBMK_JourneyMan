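; BP_PoisonShroom is a kart item that temporarily slows the first player's kart.
; Its PoisonShroom event raises a flag on the kart, waits two seconds, then clears it and sets current speed to the default max.
; While the flag is set, Tick passes through a DoOnce that drops speed below the current max once.
; The event resets that DoOnce after restoring speed.
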(event Custom|PoisonShroom
  (bind _asbp_kart (Utilities|Casting|CastToBP_Kart (Game|Player|GetPlayerPawn 0)))
  (Variables|/Game/JMan_Folder/Kart_Engine/NewTestKart/BP_Kart.BP_Kart_C|SetPoison%20Shroom _asbp_kart true)
  (Utilities|FlowControl|Delay 2.0)
  (Variables|/Game/JMan_Folder/Kart_Engine/NewTestKart/BP_Kart.BP_Kart_C|SetPoison%20Shroom _asbp_kart false)
  (Variables|/Game/JMan_Folder/Kart_Engine/NewTestKart/BP_Kart.BP_Kart_C|SetCurrent%20Speed _asbp_kart (Variables|/Game/JMan_Folder/Kart_Engine/NewTestKart/BP_Kart.BP_Kart_C|GetDefault%20Max%20Speed _asbp_kart))
  (Utilities|FlowControl|DoOnce false) ; enters at Reset
)

(event EventTick
  (params (DeltaSeconds :type Float%20%28single-precision%29))
  (bind _asbp_kart (Utilities|Casting|CastToBP_Kart (Game|Player|GetPlayerPawn 0)))
  (if (Variables|/Game/JMan_Folder/Kart_Engine/NewTestKart/BP_Kart.BP_Kart_C|GetPoison%20Shroom _asbp_kart)
    (Utilities|FlowControl|DoOnce false
      (:Completed
        (Variables|/Game/JMan_Folder/Kart_Engine/NewTestKart/BP_Kart.BP_Kart_C|SetCurrent%20Speed _asbp_kart (- (Variables|/Game/JMan_Folder/Kart_Engine/NewTestKart/BP_Kart.BP_Kart_C|GetCurrent%20Max%20Speed _asbp_kart) 2e+01))))))

(fn ConstructionScript)