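; BP_GreenShell is a green golf ball player item that destroys itself when its collision overlaps an actor tagged "AI".
; The BallLaunch event is empty.
; Launch logic that would apply a forward impulse along BallArrow to the Ball, then destroy the actor after a delay, is disconnected and never runs.
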(event OnComponentBeginOverlap(Collision)
  (params (OverlappedComponent :type Primitive%20Component%20Object%20Reference) (OtherActor :type Actor%20Object%20Reference) (OtherComp :type Primitive%20Component%20Object%20Reference) (OtherBodyIndex :type Integer) (bFromSweep :type Boolean) (SweepResult :type Hit%20Result%20Structure%20%28by%20ref%29))
  (if (Actor|ActorHasTag OtherActor "AI")
    (Actor|DestroyActor)))

(event Custom|BallLaunch
  ;[0.6292 0 1] Fiona - Initial Launch of Green Golf Ball - if hits no player/banana destroys self after 8 seconds
)

(fn ConstructionScript)