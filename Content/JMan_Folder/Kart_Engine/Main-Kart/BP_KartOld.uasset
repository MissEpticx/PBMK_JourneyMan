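; Player-driven kart prototype that moves and steers a Cube by setting its transform directly, with an orbiting spring-arm camera.
; Forward input steps CurrentSpeed by Acceleration toward forward, reverse or rest, then moves the Cube along the Arrow's forward vector, without sweep or delta time.
; Steering adds yaw only while moving, dividing input by a sign-matched speed, so both input signs yaw the same direction.
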(event Input|AxisEvents|InputAxisForward
  (params (AxisValue :type Float%20%28single-precision%29))
  (bind _current_speed (Variables|Default|GetCurrent%20Speed))
  (bind _cube (Variables|Default|GetCube))
  ;[1 1 1] move forwards / backwards
  (if (> AxisValue 0.0)
    (CallFunction|Accelerate (Variables|Default|GetMax%20Speed))
    (if (== (Variables|Default|GetCurrent%20Speed) 0.0) :!label _label
      (Variables|Default|SetIs%20Moving false)
      (else
        (Variables|Default|SetIs%20Moving true)))
    (Transformation|SetWorldLocation _cube (+ (Transformation|GetWorldLocation _cube) (* (Math|Vector|GetForwardVector (Variables|Default|GetArrow)) (Variables|Default|GetCurrent%20Speed))) false false)
    (elif (< AxisValue 0.0)
      (CallFunction|Deccelerate (* -1 (Variables|Default|GetMax%20Speed)))
      (goto _label)
      (elif (> _current_speed 0.0)
        (CallFunction|Deccelerate 0.0)
        (goto _label)
        (elif (< _current_speed 0.0)
          (CallFunction|Accelerate 0.0)
          (goto _label))))))

(event Input|AxisEvents|InputAxisTurning
  (params (AxisValue :type Float%20%28single-precision%29))
  (bind _cube (Variables|Default|GetCube))
  (bind _returnvalue (Transformation|GetWorldRotation _cube))
  ;[1 1 1] turn left / right
  (if (< (stale Input|AxisEvents|InputAxisForward AxisValue) 0.0)
    (Variables|Default|SetSteering%20Speed (* -1 (Variables|Default|GetDefualt%20Steer%20Speed)))
    (else
      (Variables|Default|SetSteering%20Speed (Variables|Default|GetDefualt%20Steer%20Speed))))
  (if (Variables|Default|GetIs%20Moving)
    (Transformation|SetWorldRotation _cube (Math|Rotator|MakeRotator (.roll _returnvalue) (.pitch _returnvalue) (+ (.yaw _returnvalue) (/ AxisValue (Variables|Default|GetSteering%20Speed)))) false false)))

(event Input|MouseEvents|MouseX
  (params (AxisValue :type Float%20%28single-precision%29))
  ;[1 1 1] pan camera
  (Transformation|AddRelativeRotation (Variables|Default|GetSpringArm) (Math|Rotator|MakeRotator 0.0 0.0 AxisValue) false false))

(event Input|MouseEvents|MouseY
  (params (AxisValue :type Float%20%28single-precision%29))
  ;[1 1 1] pan camera
  (Transformation|AddRelativeRotation (Variables|Default|GetSpringArm) (Math|Rotator|MakeRotator 0.0 AxisValue 0.0) false false))

(event Input|GamepadEvents|GamepadRightX
  (params (AxisValue :type Float%20%28single-precision%29))
  ;[1 1 1] pan camera
  (Transformation|AddRelativeRotation (Variables|Default|GetSpringArm) (Math|Rotator|MakeRotator 0.0 0.0 AxisValue) false false))

(event Input|GamepadEvents|GamepadRightY
  (params (AxisValue :type Float%20%28single-precision%29))
  ;[1 1 1] pan camera
  (Transformation|AddRelativeRotation (Variables|Default|GetSpringArm) (Math|Rotator|MakeRotator 0.0 (* AxisValue -1.0) 0.0) false false))

(fn ConstructionScript)

(fn Deccelerate
  (params (Min%20Speed :type Float%20%28single-precision%29))
  (if (not (< (Variables|Default|GetCurrent%20Speed) Min%20Speed))
    (Variables|Default|SetCurrent%20Speed (- (Variables|Default|GetCurrent%20Speed) (Variables|Default|GetAcceleration)))))

(fn Accelerate
  (params (Max%20Speed :type Float%20%28single-precision%29))
  (if (not (> (Variables|Default|GetCurrent%20Speed) Max%20Speed))
    (Variables|Default|SetCurrent%20Speed (+ (Variables|Default|GetCurrent%20Speed) (Variables|Default|GetAcceleration)))))