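; BP_HoverComponent is a hover suspension point that pushes its owning BP_KartOld away from the surface beneath it.
; Each tick it line-traces down its own up vector to the hover distance, with debug drawing on.
; On a hit, it applies a spring-damper force to the kart's root primitive at the component's location, using compression and its rate of change since the last recorded hit.
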(event EventBeginPlay
  (bind _asbp_kart (Utilities|Casting|CastToBP_KartOld (Components|GetOwner)))
  (Variables|Default|SetParentVehicle _asbp_kart))

(event EventTick
  (params (DeltaSeconds :type Float%20%28single-precision%29))
  (bind _returnvalue (Transformation|GetWorldLocation))
  (Utilities|IsValid (Variables|Default|GetParentVehicle)
    (:Is%20Valid
      (bind (_outhit _returnvalue_2) (Collision|LineTraceByChannel _returnvalue (- _returnvalue (* (Math|Vector|GetUpVector) (Variables|Default|GetHoverDistance))) "TraceTypeQuery1" false 0 "ForOneFrame"))
      (if _returnvalue_2
        (bind _output_get (Variables|Default|SetHoverDelta (- (Variables|Default|GetHoverDistance) (.Distance (Collision|BreakHitResult _outhit)))))
        (Class|PrimitiveComponent|AddForceatLocation (.AsPrimitive%20Component (Utilities|Casting|CastToPrimitiveComponent (Variables|/Script/Engine.Actor|GetRootComponent (Variables|Default|GetParentVehicle)))) (* (Math|Vector|GetUpVector) (+ (* (/ (- _output_get (Variables|Default|GetPreviousHoverDelta)) (Utilities|Time|GetWorldDeltaSeconds)) (Variables|Default|GetDampingCoefficient)) (* _output_get (Variables|Default|GetSpringCoefficient)))) (Transformation|GetWorldLocation) "None")
        (Variables|Default|SetPreviousHoverDelta (Variables|Default|GetHoverDelta))))
    (:Is%20Not%20Valid
      (Development|PrintString "Not valiud"))))