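; Player-controlled kart character that drives, steers and jumps using character movement, with jump noted as a possible future drift.
; Forward input moves it along Arrow1's forward vector and sets IsMoving, which gates steering.
; Steering adds yaw to OriginPoint, with input divided by SteeringSpeed, so higher values turn slower.
; Mouse and right stick rotate the SpringArm camera, with only the stick's vertical axis inverted.
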(event Input|ActionEvents|InputActionJump
  (params (Key :type Key%20Structure :default "None"))
  ;[1 1 1] jump (can use for drift later)
  (:Pressed
    (Character|Jump)))

(event Input|AxisEvents|InputAxisForward
  (params (AxisValue :type Float%20%28single-precision%29))
  ;[1 1 1] move forwards / backwards
  (if (== AxisValue 0.0)
    (Variables|Default|SetIs%20Moving false)
    (else
      (Variables|Default|SetIs%20Moving true)
      (Pawn|Input|AddMovementInput (* (Math|Vector|GetForwardVector (Variables|Default|GetArrow1)) (Variables|Default|GetMove%20Speed)) AxisValue false))))

(event Input|AxisEvents|InputAxisTurning
  (params (AxisValue :type Float%20%28single-precision%29))
  (bind _originpoint (Variables|Default|GetOriginPoint))
  (bind _returnvalue (Transformation|GetWorldRotation _originpoint))
  ;[1 1 1] turn left / right
  (if (Variables|Default|GetIs%20Moving)
    (Transformation|SetWorldRotation _originpoint (Math|Rotator|MakeRotator (.roll _returnvalue) (.pitch _returnvalue) (+ (.yaw _returnvalue) (/ AxisValue (Variables|Default|GetSteering%20Speed)))) false false)))

(event Input|MouseEvents|MouseX
  (params (AxisValue :type Float%20%28single-precision%29))
  ;[1 1 1] pan camera
  (Transformation|AddRelativeRotation (Variables|Default|GetSpring%20arm) (Math|Rotator|MakeRotator 0.0 0.0 AxisValue) false false))

(event Input|MouseEvents|MouseY
  (params (AxisValue :type Float%20%28single-precision%29))
  ;[1 1 1] pan camera
  (Transformation|AddRelativeRotation (Variables|Default|GetSpring%20arm) (Math|Rotator|MakeRotator 0.0 AxisValue 0.0) false false))

(event Input|GamepadEvents|GamepadRightX
  (params (AxisValue :type Float%20%28single-precision%29))
  ;[1 1 1] pan camera
  (Transformation|AddRelativeRotation (Variables|Default|GetSpring%20arm) (Math|Rotator|MakeRotator 0.0 0.0 AxisValue) false false))

(event Input|GamepadEvents|GamepadRightY
  (params (AxisValue :type Float%20%28single-precision%29))
  ;[1 1 1] pan camera
  (Transformation|AddRelativeRotation (Variables|Default|GetSpring%20arm) (Math|Rotator|MakeRotator 0.0 (* AxisValue -1.0) 0.0) false false))

(fn ConstructionScript)