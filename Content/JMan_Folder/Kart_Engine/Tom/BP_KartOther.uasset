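; BP_KartOther is a simple kart actor that drives itself in a straight line along the direction of its Arrow component.
; Each Tick offsets the DefaultSceneRoot world location by the arrow's forward vector times MoveSpeed, with no sweep and no delta-time scaling, so speed depends on frame rate.
; The overlap event and construction script are empty, and a root transform node is left unconnected.
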(event Collision|EventActorBeginOverlap
  (params (OtherActor :type Actor%20Object%20Reference)))

(event EventTick
  (params (DeltaSeconds :type Float%20%28single-precision%29))
  (Transformation|SetWorldLocation (Variables|Default|GetDefaultSceneRoot) (+ (Transformation|GetWorldLocation (Variables|Default|GetDefaultSceneRoot)) (* (Math|Vector|GetForwardVector (Variables|Default|GetArrow)) (Variables|Default|GetMove%20Speed))) false false))

(fn ConstructionScript)