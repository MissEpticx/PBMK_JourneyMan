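; BP_HoverComponent is a hover component for the BP_TestRaycast kart vehicle, currently performing only a ground probe.
; On BeginPlay it casts its owner to BP_TestRaycast and caches it as ParentVehicle.
; Each tick, while that reference is valid, it line traces on the Visibility channel along its local down axis for HoverDistance.
; The trace result is unused, so no hover force is applied here.
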(event EventBeginPlay
  (bind _asbp_test_raycast (Utilities|Casting|CastToBP_TestRaycast (Components|GetOwner)))
  (Variables|Default|SetParentVehicle _asbp_test_raycast))

(event EventTick
  (params (DeltaSeconds :type Float%20%28single-precision%29))
  (bind _returnvalue (Transformation|GetWorldLocation))
  (Utilities|IsValid (Variables|Default|GetParentVehicle)
    (:Is%20Valid
      (Collision|LineTraceByChannel _returnvalue (- _returnvalue (* (Math|Vector|GetUpVector) (Variables|Default|GetHoverDistance))) "TraceTypeQuery1" false 0 "None"))))