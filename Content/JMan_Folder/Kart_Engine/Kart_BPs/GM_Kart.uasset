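; GM_Kart is the kart game mode that resolves which character kart Player 1 uses.
; On BeginPlay it reads the selection flags on the KartInstance game instance through a chain of branches, checking Mario, Luigi, Peach, Bowser, Waluigi and Koopa in turn.
; The first true flag stores the matching kart Blueprint in Player1Character; this graph does no spawning itself.
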(event EventBeginPlay
  (bind _askart_instance (Utilities|Casting|CastToKartInstance (Game|GetGameInstance)))
  (if (Variables|/Game/KartInstance.KartInstance_C|GetIsMario _askart_instance)
    (Variables|Default|SetPlayer%201%20Character "/Game/JMan_Folder/Kart_Engine/Kart_BPs/Karts/BP_Mario_Kart.BP_Mario_Kart_C")
    (elif (Variables|/Game/KartInstance.KartInstance_C|GetIsLuigi _askart_instance)
      (Variables|Default|SetPlayer%201%20Character "/Game/JMan_Folder/Kart_Engine/Kart_BPs/Karts/BP_Luigi_Kart.BP_Luigi_Kart_C")
      (elif (Variables|/Game/KartInstance.KartInstance_C|GetIsPeach _askart_instance)
        (Variables|Default|SetPlayer%201%20Character "/Game/JMan_Folder/Kart_Engine/Kart_BPs/Karts/BP_Peach_Kart.BP_Peach_Kart_C")
        (elif (Variables|/Game/KartInstance.KartInstance_C|GetIsBowser _askart_instance)
          (Variables|Default|SetPlayer%201%20Character "/Game/JMan_Folder/Kart_Engine/Kart_BPs/Karts/BP_Bowser_Kart.BP_Bowser_Kart_C")
          (elif (Variables|/Game/KartInstance.KartInstance_C|GetIsWaluigi _askart_instance)
            (Variables|Default|SetPlayer%201%20Character "/Game/JMan_Folder/Kart_Engine/Kart_BPs/Karts/BP_Waluigi_Kart.BP_Waluigi_Kart_C")
            (elif (Variables|/Game/KartInstance.KartInstance_C|GetIsKoopa _askart_instance)
              (Variables|Default|SetPlayer%201%20Character "/Game/JMan_Folder/Kart_Engine/Kart_BPs/Karts/BP_KoopaTroopa_Kart.BP_KoopaTroopa_Kart_C"))))))))

(fn ConstructionScript)