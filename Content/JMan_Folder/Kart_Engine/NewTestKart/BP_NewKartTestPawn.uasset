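; Test kart pawn that drives and steers by directly moving and rotating its Box, with a spring-arm camera panned by mouse or gamepad.
; Forward and turning input only apply while grounded, as decided each tick by a short downward line trace.
; While airborne, it keeps moving horizontally at AirSpeed and a timeline levels its pitch and roll.
; Movement has no sweep or delta-time scaling.
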(event EventTick
  (params (DeltaSeconds :type Float%20%28single-precision%29))
  (bind _arrow (Variables|Default|GetArrow))
  (bind _box (Variables|Default|GetBox))
  (bind _box_2 (Variables|Default|GetBox))
  (bind _returnvalue (Math|Vector|GetForwardVector _arrow))
  (bind _returnvalue_2 (Transformation|GetWorldLocation _box_2))
  (bind _returnvalue_3 (Transformation|GetWorldRotation _box))
  ;[1 1 1] Detect if airborne
  (bind _returnvalue_4 (Collision|LineTraceByChannel (Math|Vector|MakeVector (.x _returnvalue_2) (.y _returnvalue_2) (.z _returnvalue_2)) (Math|Vector|MakeVector (.x _returnvalue_2) (.y _returnvalue_2) (- (.z _returnvalue_2) (Variables|Default|GetCheckAirborneDist))) "TraceTypeQuery1" false 0 "ForOneFrame"))
  (if _returnvalue_4
    (Variables|Default|SetIs%20Airborne false)
    (else
      (Variables|Default|SetIs%20Airborne true)
      ;[1 1 1] move forwards if in air
      (CallFunction|DriveForwards 1.0 (Math|Vector|MakeVector (.x _returnvalue) (.y _returnvalue) 0.0) (Variables|Default|GetAir%20Speed))
      ;[1 1 1] Flatten car in mid air
      (bind _newtrack_0 (Timeline|Flatten Play)
        (:Update
          (Transformation|SetWorldRotation _box (Math|Rotator|Lerp(Rotator) (Math|Rotator|MakeRotator (.roll _returnvalue_3) (.pitch _returnvalue_3) (.yaw _returnvalue_3)) (Math|Rotator|MakeRotator 0.0 0.0 (.yaw _returnvalue_3)) _newtrack_0) false false))))))

(event Input|AxisEvents|InputAxisForward
  (params (AxisValue :type Float%20%28single-precision%29))
  ;[1 1 1] forwards
  (if (not (Variables|Default|GetIs%20Airborne))
    (CallFunction|DriveForwards AxisValue (Math|Vector|GetForwardVector (Variables|Default|GetArrow)) (Variables|Default|GetSpeed))))

(event Input|AxisEvents|InputAxisTurning
  (params (AxisValue :type Float%20%28single-precision%29))
  (bind _box (Variables|Default|GetBox))
  (bind _returnvalue (Transformation|GetWorldRotation _box))
  ;[1 1 1] Turning
  (if (not (Variables|Default|GetIs%20Airborne))
    (Transformation|SetWorldRotation _box (Math|Rotator|MakeRotator (.roll _returnvalue) (.pitch _returnvalue) (+ (.yaw _returnvalue) (/ AxisValue (Variables|Default|GetSteering%20Speed)))) false false)))

(event Input|MouseEvents|MouseX
  (params (AxisValue :type Float%20%28single-precision%29))
  ;[1 1 1] Pan Camera
  (Transformation|AddRelativeRotation (Variables|Default|GetSpringArm) (Math|Rotator|MakeRotator 0.0 0.0 AxisValue) false false))

(event Input|MouseEvents|MouseY
  (params (AxisValue :type Float%20%28single-precision%29))
  ;[1 1 1] Pan Camera
  (Transformation|AddRelativeRotation (Variables|Default|GetSpringArm) (Math|Rotator|MakeRotator 0.0 AxisValue 0.0) false false))

(event Input|GamepadEvents|GamepadRightX
  (params (AxisValue :type Float%20%28single-precision%29))
  ;[1 1 1] Pan Camera
  (Transformation|AddRelativeRotation (Variables|Default|GetSpringArm) (Math|Rotator|MakeRotator 0.0 0.0 AxisValue) false false))

(event Input|GamepadEvents|GamepadRightY
  (params (AxisValue :type Float%20%28single-precision%29))
  ;[1 1 1] Pan Camera
  (Transformation|AddRelativeRotation (Variables|Default|GetSpringArm) (Math|Rotator|MakeRotator 0.0 (* AxisValue -1.0) 0.0) false false))

(fn ConstructionScript)

(fn DriveForwards
  (params (Axis :type Float%20%28single-precision%29) (Direction :type Vector) (Speed :type Float%20%28single-precision%29))
  (bind _box (Variables|Default|GetBox))
  (Transformation|SetWorldLocation _box (+ (Transformation|GetWorldLocation _box) (* (* Direction Speed) Axis)) false false))