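; Player-driven kart prototype with arcade driving, drift boosts, an orbit camera and test inputs for item effects.
; Axis inputs adjust speed and yaw, moving the Box directly without physics.
; Tick line traces detect airborne state, block front/back movement and trigger timeline side bumps, with player hits requiring GoldFlower.
; Holding drift until its timeline finishes earns a release boost; item inputs apply timed slow, ice and mushroom effects, while Hop is unimplemented.
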(event Custom|Boost
  (params (Boost%20Speed :type Float%20%28single-precision%29) (Boost%20Duration :type Float%20%28single-precision%29))
  ;[0 1 1] Boost Event
  (bind _output_get (Variables|Default|SetCurrent%20Max%20Speed Boost%20Speed))
  (Variables|Default|SetCurrent%20Speed _output_get)
  (Utilities|FlowControl|Delay Boost%20Duration)
  (bind _output_get_2 (Variables|Default|SetCurrent%20Max%20Speed (Variables|Default|GetDefault%20Max%20Speed)))
  (Variables|Default|SetCurrent%20Speed _output_get_2))

(event Custom|Hop
  ;[0 1 1] Hop Event - Works on flat , needs tweaking for ramps/bumps
)

(event EventBeginPlay
  ;[0 1 1] Set variables at start
  (Variables|Default|SetCurrent%20Max%20Speed (Variables|Default|GetDefault%20Max%20Speed)))

(event EventTick
  (params (DeltaSeconds :type Float%20%28single-precision%29))
  (bind _arrow (Variables|Default|GetArrow))
  (bind _box (Variables|Default|GetBox))
  (bind _box_2 (Variables|Default|GetBox))
  (bind _box_3 (Variables|Default|GetBox))
  (bind _box_4 (Variables|Default|GetBox))
  (bind _box_5 (Variables|Default|GetBox))
  (bind _box_6 (Variables|Default|GetBox))
  (bind _box_7 (Variables|Default|GetBox))
  (bind _box_8 (Variables|Default|GetBox))
  (bind _box_9 (Variables|Default|GetBox))
  (bind _box_10 (Variables|Default|GetBox))
  (bind _returnvalue (Transformation|GetWorldLocation _box_9))
  (bind _returnvalue_2 (Transformation|GetWorldLocation _box_10))
  (bind _returnvalue_3 (Math|Vector|GetForwardVector _arrow))
  (bind _returnvalue_4 (Transformation|GetWorldLocation _box_3))
  (bind _returnvalue_5 (Transformation|GetWorldRotation _box_2))
  (bind _returnvalue_6 (Transformation|GetWorldLocation _box_4))
  (bind _returnvalue_7 (Transformation|GetWorldLocation _box_5))
  (bind _returnvalue_8 (Transformation|GetWorldLocation _box_6))
  (bind _returnvalue_9 (Transformation|GetWorldLocation _box_7))
  (bind _returnvalue_10 (Transformation|GetWorldLocation _box_8))
  (bind _returnvalue_11 (Transformation|GetWorldLocation _box))
  (Utilities|FlowControl|Sequence
    (:then_0
      ;[0 1 1] Detect if airborne
      (bind _returnvalue_12 (Collision|LineTraceByChannel _returnvalue_6 (+ _returnvalue_6 (* (Math|Vector|GetUpVector (Variables|Default|GetArrow)) (Variables|Default|GetCheck%20Airborne%20Dist))) "TraceTypeQuery1" false 0 "ForOneFrame"))
      (if _returnvalue_12
        (Variables|Default|SetIs%20Airborne false)
        (else
          (Variables|Default|SetIs%20Airborne true)
          ;[0 1 1] Set air movement direction
          (if (< (Variables|Default|GetCurrent%20Speed) 0.0)
            (Variables|Default|SetAir%20Speed (Variables|Default|GetReverse%20Air%20Speed))
            (else
              (Variables|Default|SetAir%20Speed (Variables|Default|GetForwards%20Air%20Speed))))
          ;[0 1 1] move forwards if in air
          (CallFunction|DriveForwards (Math|Vector|MakeVector (.x _returnvalue_3) (.y _returnvalue_3) 0.0) (Variables|Default|GetAir%20Speed))
          ;[0 1 1] Flatten car in mid air
          (bind _newtrack_2 (Timeline|Flatten Play)
            (:Update
              (Transformation|SetWorldRotation _box_2 (Math|Rotator|Lerp(Rotator) (Math|Rotator|MakeRotator (.roll _returnvalue_5) (.pitch _returnvalue_5) (.yaw _returnvalue_5)) (Math|Rotator|MakeRotator 0.0 0.0 (.yaw _returnvalue_5)) _newtrack_2) false false))))))
    (:then_1
      ;[0 1 1] Left Side Collisions
      ;;[0 1 1] check if left side hits anything
      (bind (_outhit _returnvalue_13) (Collision|LineTraceByChannel _returnvalue_8 (+ _returnvalue_8 (* (Math|Vector|GetRightVector (Variables|Default|GetArrow)) (* -1 (Variables|Default|GetCheck%20Side%20Dist)))) "TraceTypeQuery1" false 0 "None"))
      ;;[0.2543 0 1] Check for player hit
      (if _returnvalue_13
        (if (Components|ComponentHasTag (.HitComponent (Collision|BreakHitResult _outhit)) "Player")
          ;[0.307 0 1] Gold Flower Bump
          (if (Variables|Default|GetGoldFlower)
            (Variables|Default|SetBump%20Distance 5e+01)
            (bind _bumptime (Timeline|Timeline_0 PlayFromStart)
              (:Update
                (Transformation|SetWorldLocation _box_9 (Math|Vector|Lerp(Vector) _returnvalue (+ _returnvalue (* (Math|Vector|GetRightVector (Variables|Default|GetArrow)) (Variables|Default|GetBump%20Distance))) _bumptime) false false)
                (Variables|Default|SetCurrent%20Speed 0.0)
                (Variables|Default|SetBump%20Distance 1e+01))))
          (else
            ;;[0 1 1] Bump off object to the left
            (bind _bumptime_2 (Timeline|BumpLeft PlayFromStart)
              (:Update
                (Transformation|SetWorldLocation _box (Math|Vector|Lerp(Vector) _returnvalue_11 (+ _returnvalue_11 (* (Math|Vector|GetRightVector (Variables|Default|GetArrow)) (Variables|Default|GetBump%20Distance))) _bumptime_2) false false)
                (Variables|Default|SetCurrent%20Speed 0.0)))))))
    (:then_2
      ;[0 1 1] Right Side Collisions
      ;;[0 1 1] check if Right side hits anything
      (bind (_outhit_2 _returnvalue_14) (Collision|LineTraceByChannel _returnvalue_9 (+ _returnvalue_9 (* (Math|Vector|GetRightVector (Variables|Default|GetArrow)) (Variables|Default|GetCheck%20Side%20Dist))) "TraceTypeQuery1" false 0 "None"))
      ;;[0.2543 0 1] Check for player hit
      (if _returnvalue_14
        (if (Components|ComponentHasTag (.HitComponent (Collision|BreakHitResult _outhit_2)) "Player")
          ;[0.307 0 1] Gold Flower Bump
          (if (Variables|Default|GetGoldFlower)
            (Variables|Default|SetBump%20Distance 5e+01)
            (bind _bumptime_3 (Timeline|Timeline_2 PlayFromStart)
              (:Update
                (Transformation|SetWorldLocation _box_8 (Math|Vector|Lerp(Vector) _returnvalue_10 (+ _returnvalue_10 (* (Math|Vector|GetRightVector (Variables|Default|GetArrow)) (* -1 (Variables|Default|GetBump%20Distance)))) _bumptime_3) false false)
                (Variables|Default|SetCurrent%20Speed 0.0)
                (Variables|Default|SetBump%20Distance 1e+01))))
          (else
            ;;[0 1 1] Bump off object to the right
            (bind _bumptime_4 (Timeline|BumpRight PlayFromStart)
              (:Update
                (Transformation|SetWorldLocation _box_10 (Math|Vector|Lerp(Vector) _returnvalue_2 (+ _returnvalue_2 (* (Math|Vector|GetRightVector (Variables|Default|GetArrow)) (* -1 (Variables|Default|GetBump%20Distance)))) _bumptime_4) false false)
                (Variables|Default|SetCurrent%20Speed 0.0)))))))
    (:then_3
      ;[0 1 1] Front Collisions
      ;;[0 1 1] check if Front side hits anything
      (bind _returnvalue_15 (Collision|LineTraceByChannel _returnvalue_7 (+ _returnvalue_7 (* (Math|Vector|GetForwardVector (Variables|Default|GetArrow)) (Variables|Default|GetCheck%20Front%20Dist))) "TraceTypeQuery1" false 0 "None"))
      (if _returnvalue_15
        (Variables|Default|SetFront%20Hit true)
        (if (> (Variables|Default|GetCurrent%20Speed) 0.0)
          (Variables|Default|SetCurrent%20Speed 0.0))
        (else
          (Variables|Default|SetFront%20Hit false))))
    (:then_4
      ;[0 1 1] Back Collisions
      ;;[0 1 1] check if Front side hits anything
      (bind _returnvalue_16 (Collision|LineTraceByChannel _returnvalue_4 (+ _returnvalue_4 (* (Math|Vector|GetForwardVector (Variables|Default|GetArrow)) (* -1 (Variables|Default|GetCheck%20Front%20Dist)))) "TraceTypeQuery1" false 0 "None"))
      (if _returnvalue_16
        (Variables|Default|SetBack%20Hit true)
        (if (< (Variables|Default|GetCurrent%20Speed) 0.0)
          (Variables|Default|SetCurrent%20Speed 0.0))
        (else
          (Variables|Default|SetBack%20Hit false))))
    (:then_5
      ;[0.2118 0 1] Poison Shroom Effect
      (if (Variables|Default|GetPoison%20Shroom)
        (Utilities|FlowControl|DoOnce false
          (:Completed
            (Variables|Default|SetCurrent%20Max%20Speed (- (Variables|Default|GetCurrent%20Max%20Speed) 2e+01))))))
    (:then_6
      ;[0.2583 0 1] Ice Flower Slide
      (if (Variables|Default|GetIcy)
        (Utilities|FlowControl|DoOnce false
          (:Completed
            (bind _output_get (Variables|Default|SetIcySpeed (Variables|Default|GetCurrent%20Speed)))
            (CallFunction|DriveForwards (Math|Vector|GetForwardVector (Variables|Default|GetArrow)) _output_get)))))))

(event Input|ActionEvents|InputActionDrift
  (params (Key :type Key%20Structure :default "None"))
  ;[0 1 1] Very basic drift functionality
  (:Pressed
    (if (> (Variables|Default|GetCurrent%20Speed) 0.0)
      (if (== (Variables|Default|GetCurrent%20Direction) -1.0)
        (Variables|Default|SetDrifting%20Direction -1.0)
        (Variables|Default|SetBase%20Steering%20Speed 1.2 :!label _label)
        (Variables|Default|SetIs%20Drifting true)
        (Development|PrintString "Drifting")
        (CallFunction|Hop)
        (Timeline|Timeline_1 PlayFromStart
          (:Finished
            (Development|PrintString "Boosted")
            (Variables|Default|SetIs%20Boosted true)))
        (elif (== (Variables|Default|GetCurrent%20Direction) 1.0)
          (Variables|Default|SetDrifting%20Direction 1.0)
          (goto _label)))))
  (:Released
    (Variables|Default|SetDrifting%20Direction 0.0)
    (Variables|Default|SetBase%20Steering%20Speed 1.2)
    (Variables|Default|SetIs%20Drifting false)
    (if (Variables|Default|GetIs%20Boosted)
      (CallFunction|Boost (Variables|Default|GetBoost%20Speed) (Variables|Default|GetBoost%20Duration))
      (Variables|Default|SetIs%20Boosted false)
      (Timeline|Timeline_1 Stop)
      (else
        (Timeline|Timeline_1 Stop)))))

(event Input|ActionEvents|InputActionDaisyItem
  (params (Key :type Key%20Structure :default "None"))
  ;[0.2217 0 1] Poison Shroom Trigger
  (:Pressed
    (Variables|Default|SetPoison%20Shroom true)
    (Utilities|FlowControl|Delay 2.0)
    (Variables|Default|SetPoison%20Shroom false)
    (Variables|Default|SetCurrent%20Max%20Speed (Variables|Default|GetDefault%20Max%20Speed))
    ;[0.2118 0 1] Poison Shroom Effect
    (Utilities|FlowControl|DoOnce false) ; enters at Reset
  ))

(event Input|ActionEvents|InputActionDaisyItem2
  (params (Key :type Key%20Structure :default "None"))
  ;[0.2186 0 1] Ice Flower Trigger
  (:Pressed
    (Variables|Default|SetIcy true)
    (Utilities|FlowControl|Delay 2.0)
    (Variables|Default|SetIcy false)))

(event Input|ActionEvents|InputActionDaisyItem3
  (params (Key :type Key%20Structure :default "None"))
  ;[0.2581 0 1] Mushroom
  (:Pressed
    (Variables|Default|SetCurrent%20Max%20Speed 5e+01)
    (Variables|Default|SetCurrent%20Speed (+ (Variables|Default|GetCurrent%20Speed) 2e+01))
    (Utilities|FlowControl|Delay 2.0)
    (Variables|Default|SetCurrent%20Max%20Speed (Variables|Default|GetDefault%20Max%20Speed))))

(event Input|AxisEvents|InputAxisForward
  (params (AxisValue :type Float%20%28single-precision%29))
  (bind _acceleration (Variables|Default|GetAcceleration))
  (bind _current_speed (Variables|Default|GetCurrent%20Speed))
  ;[0 1 1] Driving (With Acceleration)
  (if (not (Variables|Default|GetIs%20Airborne))
    (if (> AxisValue 0.0)
      (if (not (Variables|Default|GetFront%20Hit))
        (CallFunction|Accelerate (Variables|Default|GetCurrent%20Max%20Speed))
        (CallFunction|DriveForwards (Math|Vector|GetForwardVector (Variables|Default|GetArrow)) (Variables|Default|GetCurrent%20Speed) :!label _label))
      (elif (< AxisValue 0.0)
        (if (not (Variables|Default|GetBack%20Hit))
          (CallFunction|Deccelerate (* -1 (Variables|Default|GetCurrent%20Max%20Speed)))
          (goto _label))
        (elif (> _current_speed _acceleration)
          (if (not (Variables|Default|GetBack%20Hit))
            (CallFunction|Deccelerate 0.0)
            (goto _label))
          (elif (< _current_speed _acceleration)
            (if (not (Variables|Default|GetFront%20Hit))
              (CallFunction|Accelerate 0.0)
              (goto _label))))))))

(event Input|AxisEvents|InputAxisTurning
  (params (AxisValue :type Float%20%28single-precision%29))
  (bind _box (Variables|Default|GetBox))
  (bind _returnvalue (Transformation|GetWorldRotation _box))
  ;[0 1 1] Turning
  (if (Variables|Default|GetIs%20Drifting)
    ;;[0 1 1] Change turning input when drifting
    (if (== (Variables|Default|GetCurrent%20Direction) -1.0)
      (Variables|Default|SetSteering%20Speed (+ (Variables|Default|GetSteering%20Speed) (* (Variables|Default|GetSteering%20Accelleration) AxisValue)))
      (else
        (Variables|Default|SetSteering%20Speed (- (Variables|Default|GetSteering%20Speed) (* (Variables|Default|GetSteering%20Accelleration) AxisValue)))))
    (Transformation|SetWorldRotation _box (Math|Rotator|MakeRotator (.roll _returnvalue) (.pitch _returnvalue) (+ (.yaw _returnvalue) (/ (Variables|Default|GetCurrent%20Direction) (Variables|Default|GetSteering%20Speed)))) false false :!label _label)
    (else
      (Variables|Default|SetCurrent%20Direction AxisValue)
      (if (== (Variables|Default|GetDrifting%20Direction) 0.0)
        _
        (else
          (Variables|Default|SetCurrent%20Direction (Variables|Default|GetDrifting%20Direction))))
      (if (not (or (Variables|Default|GetIs%20Airborne) (== (Variables|Default|GetCurrent%20Speed) 0.0)))
        (if (not (Variables|Default|GetIcy))
          (if (< (Variables|Default|GetCurrent%20Speed) 0.0)
            (Variables|Default|SetSteering%20Speed (* -1 (Variables|Default|GetBase%20Steering%20Speed)))
            (goto _label)
            (else
              (Variables|Default|SetSteering%20Speed (Variables|Default|GetBase%20Steering%20Speed))
              (goto _label))))))))

(event Input|MouseEvents|MouseX
  (params (AxisValue :type Float%20%28single-precision%29))
  ;[0 1 1] Pan Camera
  (Transformation|AddRelativeRotation (Variables|Default|GetSpringArm) (Math|Rotator|MakeRotator 0.0 0.0 AxisValue) false false))

(event Input|MouseEvents|MouseY
  (params (AxisValue :type Float%20%28single-precision%29))
  ;[0 1 1] Pan Camera
  (Transformation|AddRelativeRotation (Variables|Default|GetSpringArm) (Math|Rotator|MakeRotator 0.0 AxisValue 0.0) false false))

(event Input|GamepadEvents|GamepadRightX
  (params (AxisValue :type Float%20%28single-precision%29))
  ;[0 1 1] Pan Camera
  (Transformation|AddRelativeRotation (Variables|Default|GetSpringArm) (Math|Rotator|MakeRotator 0.0 0.0 AxisValue) false false))

(event Input|GamepadEvents|GamepadRightY
  (params (AxisValue :type Float%20%28single-precision%29))
  ;[0 1 1] Pan Camera
  (Transformation|AddRelativeRotation (Variables|Default|GetSpringArm) (Math|Rotator|MakeRotator 0.0 (* AxisValue -1.0) 0.0) false false))

(fn ConstructionScript)

(fn DriveForwards
  (params (Direction :type Vector) (Speed :type Float%20%28single-precision%29))
  (bind _box (Variables|Default|GetBox))
  (Transformation|SetWorldLocation _box (+ (Transformation|GetWorldLocation _box) (* Direction Speed)) false false))

(fn Accelerate
  (params (Max%20Speed :type Float%20%28single-precision%29))
  (if (>= (Variables|Default|GetCurrent%20Speed) Max%20Speed)
    (Variables|Default|SetCurrent%20Speed Max%20Speed)
    (else
      (Variables|Default|SetCurrent%20Speed (+ (Variables|Default|GetCurrent%20Speed) (Variables|Default|GetAcceleration))))))

(fn Deccelerate
  (params (Min%20Speed :type Float%20%28single-precision%29))
  (if (<= (Variables|Default|GetCurrent%20Speed) Min%20Speed)
    (Variables|Default|SetCurrent%20Speed Min%20Speed)
    (else
      (Variables|Default|SetCurrent%20Speed (- (Variables|Default|GetCurrent%20Speed) (Variables|Default|GetAcceleration))))))